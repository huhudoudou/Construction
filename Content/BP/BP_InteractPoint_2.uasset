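; BP_InteractPoint_2 is a clickable interaction point that acts as one step in a chain of such points.
; On BeginPlay it finds and caches the level's BP_Ground actor.
; Clicking its static mesh makes the ground visible and calls its Wajueji function, then spawns BP_InteractPoint_3 at a hardcoded location and destroys itself.
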(event OnClicked(StaticMesh)
  (params (TouchedComponent :type Primitive%20Component%20Object%20Reference) (ButtonPressed :type Key%20Structure :default "None"))
  (bind _groundref (Variables|Default|GetGroundRef))
  (Default|SetVisible _groundref true)
  (Default|Wajueji _groundref)
  (Game|SpawnActorfromClass "/Game/BP/BP_InteractPoint_3.BP_InteractPoint_3_C" (Math|Transform|MakeTransform "-600.000000,1200.000000,0.000000" "0, 0, 0" "1.000000,1.000000,1.000000") "Undefined" "MultiplyWithRoot" 0 0)
  (Actor|DestroyActor))

(event EventBeginPlay
  (|CallParentFunction)
  (bind _returnvalue (Actor|GetActorOfClass "/Game/BP/BP_Ground.BP_Ground_C"))
  (Utilities|IsValid _returnvalue
    (:Is%20Valid
      (Variables|Default|SetGroundRef _returnvalue))))

(event Collision|EventActorBeginOverlap
  (params (OtherActor :type Actor%20Object%20Reference))
  (|CallParentFunction OtherActor) ; This node is disabled and will not be called.\nDrag off pins to build functionality.
)

(event EventTick
  (params (DeltaSeconds :type Float%20%28single-precision%29))
  (|CallParentFunction DeltaSeconds) ; This node is disabled and will not be called.\nDrag off pins to build functionality.
)

(fn ConstructionScript
  (|CallParentFunction))