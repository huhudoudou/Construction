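; BP_InteractPoint_3 is a clickable interaction point that plays a staged, multi-step cinematic on the BP_03 actor found at BeginPlay.
; Clicking its static mesh chains seven of that actor's ActorSequences with hardcoded delays, hiding its widget and toggling visibility of Guandao and other components along the way.
; When the chain ends, it spawns BP_04 at a fixed location and destroys itself.
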(event OnClicked(StaticMesh)
  (params (TouchedComponent :type Primitive%20Component%20Object%20Reference) (ButtonPressed :type Key%20Structure :default "None"))
  (bind _p3ref (Variables|Default|GetP3Ref))
  (bind _p3ref_2 (Variables|Default|GetP3Ref))
  (Class|ActorSequenceComponent|PlaySequence (Variables|/Game/BP/BP_03.BP_03_C|GetActorSequence1 _p3ref))
  (Utilities|FlowControl|Delay 1.6)
  (Class|ActorSequenceComponent|PlaySequence (Variables|/Game/BP/BP_03.BP_03_C|GetActorSequence2 _p3ref))
  (Rendering|SetVisibility (Variables|/Game/BP/BP_03.BP_03_C|GetWidget _p3ref) false false)
  (Utilities|FlowControl|Delay 5.0)
  (Rendering|SetVisibility (Variables|/Game/BP/BP_03.BP_03_C|Getguandao_01_5 (Variables|Default|GetP3Ref)) true false)
  (Class|ActorSequenceComponent|PlaySequence (Variables|/Game/BP/BP_03.BP_03_C|GetActorSequence3 _p3ref))
  (Utilities|FlowControl|Delay 2.24)
  (Class|ActorSequenceComponent|PlaySequence (Variables|/Game/BP/BP_03.BP_03_C|GetActorSequence4 _p3ref))
  (Utilities|FlowControl|Delay 1e+01)
  (Class|ActorSequenceComponent|PlaySequence (Variables|/Game/BP/BP_03.BP_03_C|GetActorSequence5 _p3ref_2))
  (Utilities|FlowControl|Delay 9.05)
  (Rendering|SetVisibility (Variables|/Game/BP/BP_03.BP_03_C|Get016_2 _p3ref_2) false false)
  (Class|ActorSequenceComponent|PlaySequence (Variables|/Game/BP/BP_03.BP_03_C|GetActorSequence6 _p3ref_2))
  (Utilities|FlowControl|Delay 10.7)
  (Class|ActorSequenceComponent|PlaySequence (Variables|/Game/BP/BP_03.BP_03_C|GetActorSequence7 _p3ref_2))
  (Utilities|FlowControl|Delay 3.7)
  (Game|SpawnActorfromClass "/Game/BP_04.BP_04_C" (Math|Transform|MakeTransform "16.000000,8.000000,5.000000" "0, 0, 0" "1.000000,1.000000,1.000000") "Undefined" "MultiplyWithRoot" 0 0)
  (Actor|DestroyActor))

(event EventBeginPlay
  (|CallParentFunction)
  (bind _returnvalue (Actor|GetActorOfClass "/Game/BP/BP_03.BP_03_C"))
  (Utilities|IsValid _returnvalue
    (:Is%20Valid
      (Variables|Default|SetP3Ref _returnvalue))))

(event Collision|EventActorBeginOverlap
  (params (OtherActor :type Actor%20Object%20Reference))
  (|CallParentFunction OtherActor) ; This node is disabled and will not be called.\nDrag off pins to build functionality.
)

(event EventTick
  (params (DeltaSeconds :type Float%20%28single-precision%29))
  (|CallParentFunction DeltaSeconds) ; This node is disabled and will not be called.\nDrag off pins to build functionality.
)

(fn ConstructionScript
  (|CallParentFunction))