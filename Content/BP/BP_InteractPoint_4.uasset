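; Clickable interaction point for step 4 of a chained sequence, handing off to step 5 when done.
; BeginPlay caches the BP_04 and BP_Ground actors in the level.
; Clicking the mesh plays BP_04's ActorSequences on fixed delays, hiding the ground's ladder mesh partway through.
; It destroys BP_04 immediately after starting the fourth sequence, spawns BP_05 and BP_InteractPoint_5, then destroys itself.
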(event OnClicked(StaticMesh)
  (params (TouchedComponent :type Primitive%20Component%20Object%20Reference) (ButtonPressed :type Key%20Structure :default "None"))
  (bind _04ref (Variables|Default|Get04Ref))
  (Class|ActorSequenceComponent|PlaySequence (Variables|/Game/BP/BP_04.BP_04_C|GetActorSequence1 _04ref))
  (Utilities|FlowControl|Delay 14.0)
  (Rendering|SetVisibility (Variables|/Game/BP/BP_Ground.BP_Ground_C|GetSM_Ladder (Variables|Default|GetP2Ref)) false false)
  (Class|ActorSequenceComponent|PlaySequence (Variables|/Game/BP/BP_04.BP_04_C|GetActorSequence2 _04ref))
  (Utilities|FlowControl|Delay 7.0)
  (Class|ActorSequenceComponent|PlaySequence (Variables|/Game/BP/BP_04.BP_04_C|GetActorSequence3 _04ref))
  (Utilities|FlowControl|Delay 11.0)
  (Class|ActorSequenceComponent|PlaySequence (Variables|/Game/BP/BP_04.BP_04_C|GetActorSequence4 _04ref))
  (Actor|DestroyActor (Variables|Default|Get04Ref))
  (Game|SpawnActorfromClass "/Game/BP/BP_05.BP_05_C" (Math|Transform|MakeTransform "18.000000,8.000000,5.000000" "0, 0, 0" "1.000000,1.000000,1.000000") "Undefined" "MultiplyWithRoot" 0 0)
  (Game|SpawnActorfromClass "/Game/BP/BP_InteractPoint_5.BP_InteractPoint_5_C" (Math|Transform|MakeTransform "400.000000,1200.000000,0.000000" "0, 0, 0" "1.000000,1.000000,1.000000") "Undefined" "MultiplyWithRoot" 0 0)
  (Actor|DestroyActor))

(event EventBeginPlay
  (|CallParentFunction)
  (bind _returnvalue (Actor|GetActorOfClass "/Game/BP/BP_04.BP_04_C"))
  (Utilities|IsValid _returnvalue
    (:Is%20Valid
      (Variables|Default|Set04Ref _returnvalue)
      (bind _returnvalue_2 (Actor|GetActorOfClass "/Game/BP/BP_Ground.BP_Ground_C"))
      (Utilities|IsValid _returnvalue_2
        (:Is%20Valid
          (Variables|Default|SetP2Ref _returnvalue_2))))))

(event Collision|EventActorBeginOverlap
  (params (OtherActor :type Actor%20Object%20Reference))
  (|CallParentFunction OtherActor) ; This node is disabled and will not be called.\nDrag off pins to build functionality.
)

(event EventTick
  (params (DeltaSeconds :type Float%20%28single-precision%29))
  (|CallParentFunction DeltaSeconds) ; This node is disabled and will not be called.\nDrag off pins to build functionality.
)

(fn ConstructionScript
  (|CallParentFunction))