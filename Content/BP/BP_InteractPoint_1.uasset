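; BP_InteractPoint_1 is a one-shot clickable interaction point that triggers an animated sequence on the BP_01 actor.
; BeginPlay finds and caches the BP_01 instance in the level.
; Clicking the static mesh plays BP_01's Actor Sequence and hides the mesh.
; After a fixed 30-second delay, it hides BP_01's whole component hierarchy and destroys itself, leaving BP_01 hidden but not destroyed.
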(event OnClicked(StaticMesh)
  (params (TouchedComponent :type Primitive%20Component%20Object%20Reference) (ButtonPressed :type Key%20Structure :default "None"))
  (Class|ActorSequenceComponent|PlaySequence (Variables|/Game/BP_01.BP_01_C|GetActorSequence (Variables|Default|Get01Ref)))
  (Rendering|SetVisibility (Variables|Default|GetStaticMesh) false false)
  (Utilities|FlowControl|Delay 3e+01)
  (Rendering|SetVisibility (Variables|/Game/BP_01.BP_01_C|GetDefaultSceneRoot (Variables|Default|Get01Ref)) false true)
  (Actor|DestroyActor))

(event EventBeginPlay
  (|CallParentFunction)
  (bind _returnvalue (Actor|GetActorOfClass "/Game/BP_01.BP_01_C"))
  (if (Utilities|IsValid _returnvalue)
    (Variables|Default|Set01Ref _returnvalue)))

(event Collision|EventActorBeginOverlap
  (params (OtherActor :type Actor%20Object%20Reference))
  (|CallParentFunction OtherActor) ; This node is disabled and will not be called.\nDrag off pins to build functionality.
)

(fn ConstructionScript
  (|CallParentFunction))