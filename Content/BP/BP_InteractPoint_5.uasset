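; BP_InteractPoint_5 is a one-shot clickable interaction point that triggers an animation on the BP_05 actor.
; On BeginPlay it finds BP_05 in the level and caches a reference to it.
; Clicking its static mesh plays that actor's ActorSequence1 at half speed, then destroys the interaction point so it cannot be used again.
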(event OnClicked(StaticMesh)
  (params (TouchedComponent :type Primitive%20Component%20Object%20Reference) (ButtonPressed :type Key%20Structure :default "None"))
  (bind _05ref (Variables|Default|Get05Ref))
  (bind _actorsequence1 (Variables|/Game/BP/BP_05.BP_05_C|GetActorSequence1 _05ref))
  (Components|Timeline|SetPlayRate (Variables|/Script/ActorSequence.ActorSequenceComponent|GetSequencePlayer _actorsequence1) 0.5)
  (Class|ActorSequenceComponent|PlaySequence _actorsequence1)
  (Actor|DestroyActor))

(event EventBeginPlay
  (|CallParentFunction)
  (bind _returnvalue (Actor|GetActorOfClass "/Game/BP/BP_05.BP_05_C"))
  (Utilities|IsValid _returnvalue
    (:Is%20Valid
      (Variables|Default|Set05Ref _returnvalue))))

(event Collision|EventActorBeginOverlap
  (params (OtherActor :type Actor%20Object%20Reference))
  (|CallParentFunction OtherActor) ; This node is disabled and will not be called.\nDrag off pins to build functionality.
)

(event EventTick
  (params (DeltaSeconds :type Float%20%28single-precision%29))
  (|CallParentFunction DeltaSeconds) ; This node is disabled and will not be called.\nDrag off pins to build functionality.
)

(fn ConstructionScript
  (|CallParentFunction))