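; BP_03 is an actor Blueprint that carries seven Actor Sequence components and starts out hidden.
; On BeginPlay it hides the default scene root and its children, then calls SetRate.
; SetRate loops over the sequence components and sets each player to half speed.
; This Blueprint's graphs neither play the sequences nor make the actor visible again.
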(event EventBeginPlay
  (Rendering|SetVisibility (Variables|Default|GetDefaultSceneRoot) false true)
  (CallFunction|SetRate))

(event Collision|EventActorBeginOverlap
  (params (OtherActor :type Actor%20Object%20Reference)))

(event EventTick
  (params (DeltaSeconds :type Float%20%28single-precision%29)))

(fn ConstructionScript)

(fn SetRate
  (for _array_element (Utilities|Array|MakeArray (Variables|Default|GetActorSequence2) (Variables|Default|GetActorSequence1) (Variables|Default|GetActorSequence4) (Variables|Default|GetActorSequence5) (Variables|Default|GetActorSequence6) (Variables|Default|GetActorSequence7) (Variables|Default|GetActorSequence3))
    (Components|Timeline|SetPlayRate (Variables|/Script/ActorSequence.ActorSequenceComponent|GetSequencePlayer _array_element) 0.5)))